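; BP_PlayerCharacter is the player character Blueprint, adding the on-screen UI and providing a weapon socket lookup.
; BeginPlay creates BP_Widget for player controller 0 and adds it to the viewport, while Tick and the construction script are empty.
; GetWeaponSocket reads WeaponClass from player pawn 0 rather than self, casts it to Weapon and returns the named socket's location on its GunWeapon.
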(event EventBeginPlay
  (bind _returnvalue (UserInterface|CreateWidget "/Game/BluePrint/BP_Widget.BP_Widget_C" (Game|GetPlayerController 0)))
  (UserInterface|Viewport|AddtoViewport _returnvalue 0))

(event EventTick
  (params (DeltaSeconds :type Float%20%28single-precision%29)))

(fn ConstructionScript)

(fn GetWeaponSocket
  (params (Socket%20Name :type Name))
  (bind _asbp_player_character (Utilities|Casting|CastToBP_PlayerCharacter (Game|Player|GetPlayerPawn 0)))
  (Utilities|IsValid (Variables|/Script/RogueDoom.PlayerCharacter|GetWeaponClass _asbp_player_character)
    (:Is%20Valid
      (bind _asweapon (Utilities|Casting|CastToWeapon (Variables|/Script/RogueDoom.PlayerCharacter|GetWeaponClass _asbp_player_character)))
      (return (Transformation|GetSocketLocation (Variables|/Script/RogueDoom.Weapon|GetGunWeapon _asweapon) Socket%20Name)))))
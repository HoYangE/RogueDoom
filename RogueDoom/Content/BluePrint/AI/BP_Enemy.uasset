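; BP_Enemy is an enemy AI Blueprint that provides two helper functions and has an empty construction script.
; Get Weapon Socket casts player pawn 0 to BP_PlayerCharacter and returns a named socket's location on that player's gun, rather than on a weapon of the enemy's own.
; Update Walk Speed sets the enemy's maximum walk speed on its Character Movement component.
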(fn ConstructionScript)

(fn GetWeaponSocket
  (params (Socket%20Name :type Name))
  (bind _asbp_player_character (Utilities|Casting|CastToBP_PlayerCharacter (Game|Player|GetPlayerPawn 0)))
  (Utilities|IsValid (Variables|/Script/RogueDoom.PlayerCharacter|GetWeaponClass _asbp_player_character)
    (:Is%20Valid
      (bind _asweapon (Utilities|Casting|CastToWeapon (Variables|/Script/RogueDoom.PlayerCharacter|GetWeaponClass _asbp_player_character)))
      (return (Transformation|GetSocketLocation (Variables|/Script/RogueDoom.Weapon|GetGunWeapon _asweapon) Socket%20Name)))))

(fn UpdateWalkSpeed
  (params (NewWalkSpeed :type Float%20%28double-precision%29))
  (Variables|/Script/Engine.CharacterMovementComponent|SetMaxWalkSpeed (Variables|Character|GetCharacterMovement) NewWalkSpeed))